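; Animated space station actor with spinning decorations, pulsing emissive lights and a vertically moving decoration.
; BeginPlay creates dynamic materials for three light groups and stores Decoration1's start location.
; Tick rotates pivots and scenes at fixed per-frame rates, and a DoOnce starts timelines driving top and surrounding lights and Decoration1's height.
; The ship take-off material is never driven, and the manual emissive and movement functions are not called here.
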(event `self.ReceiveBeginPlay`
  (bind _returnvalue (`PrimitiveComponent.CreateDynamicMaterialInstance` (`self.new_space_station`) 2 null "None"))
  (set `self.Emissive light_Around` _returnvalue)
  (set `self.Decoration1 Original location` (`SceneComponent.K2_GetComponentLocation` (`self.decoration1`)))
  (bind _returnvalue_2 (`PrimitiveComponent.CreateDynamicMaterialInstance` (`self.new_space_station`) 3 null "None"))
  (set `self.Emissive light_Ship take off` _returnvalue_2)
  (bind _returnvalue_3 (`PrimitiveComponent.CreateDynamicMaterialInstance` (`self.Cylinder`) 0 null "None"))
  (set `self.Emissive light_Top` _returnvalue_3))

(event `self.ReceiveTick`
  (params (DeltaSeconds :type "Float (single-precision)"))
  (`|ExecutionSequence`
    (:`then_0`
      (`SceneComponent.K2_AddWorldRotation` (`self.decoration4 pivot`) (struct :`Yaw` 0.5) false false)
      (`SceneComponent.K2_AddWorldRotation` (`self.decoration2 pivot`) (struct :`Yaw` 0.05) false false)
      (`SceneComponent.K2_AddWorldRotation` (`self.decoration3 pivot`) (struct :`Yaw` 0.05) false false)
      (`SceneComponent.K2_AddWorldRotation` (`self.Scene2`) (struct :`Yaw` 0.008) false false)
      (`SceneComponent.K2_AddWorldRotation` (`self.Scene3`) (struct :`Yaw` 0.0008) false false))
    (:`then_1`
      (`/Engine/EditorBlueprintResources/StandardMacros.DoOnce` false
        (:`Completed`
          (`|ExecutionSequence`
            (:`then_0`
              ;[1 1 1] Emissive light_ ship take off
              (bind (_direction _newtrack_0) (`Timeline|Timeline_0` :!via `PlayFromStart`)
                (:`Update`
                  (`MaterialInstanceDynamic.SetScalarParameterValue` (`self.Emissive light_Top`) "Emissive" (`KismetMathLibrary.Lerp` 5.0 500.0 _newtrack_0)))))
            (:`then_1`
              ;[1 1 1] Emissive Light around station
              (bind (_direction_2 _newtrack_0_2) (`Timeline|Timeline_1` :!via `PlayFromStart`)
                (:`Update`
                  (`MaterialInstanceDynamic.SetScalarParameterValue` (`self.Emissive light_Around`) "Emissive" (`KismetMathLibrary.Lerp` 5.0 500.0 _newtrack_0_2)))))
            (:`then_2`
              ;[1 1 1] Decoration 1 move up & down
              (bind (_direction_3 _newtrack_0_3) (`Timeline|Timeline_2` :!via `PlayFromStart`)
                (:`Update`
                  (`SceneComponent.K2_SetWorldLocation` (`self.decoration1`) (`KismetMathLibrary.VLerp` (`self.Decoration1 Original location`) (+ (`self.Decoration1 Original location`) (0.0 0.0 12000.0)) _newtrack_0_3) false false))))))))))

(fn `Decoration move up down`
  (params (`Move Decoration input` :type "StaticMeshComponent Object Reference"))
  (locals (`Move Decoration` :type "StaticMeshComponent Object Reference"))
  (bind _returnvalue (- (.z (`SceneComponent.K2_GetComponentLocation` (`local.Move Decoration`))) (.z (`self.Decoration1 Original location`))))
  (set `local.Move Decoration` `Move Decoration input`)
  (`|ExecutionSequence`
    (:`then_0`
      (if (> _returnvalue 6000.0)
        (set `self.Move up` false)))
    (:`then_1`
      (if (< _returnvalue -6000.0)
        (set `self.Move up` true)))
    (:`then_2`
      (if (`self.Move up`)
        (`SceneComponent.K2_AddWorldOffset` (`local.Move Decoration`) (0.0 0.0 50.0) false false)
        (else
          (`SceneComponent.K2_AddWorldOffset` (`local.Move Decoration`) (0.0 0.0 -50.0) false false))))))

(fn `Station Lights Emissive Change`
  (locals (`Time change rate` :type "Float (double-precision)" :default 1.0))
  (`|ExecutionSequence`
    (:`then_0`
      (if (> (`self.Time to change emissive`) 1.0)
        (set `self.Increase Emissive` false)))
    (:`then_1`
      (if (< (`self.Time to change emissive`) 0.0)
        (set `self.Increase Emissive` true)))
    (:`then_2`
      (if (> (`self.Time to change emissive`) 0.2)
        (set `local.Time change rate` 1.0)
        (else
          (set `local.Time change rate` 0.5)))
      (if (`self.Increase Emissive`)
        (set `self.Time to change emissive` (+ (`self.Time to change emissive`) (* (`GameplayStatics.GetWorldDeltaSeconds`) (`local.Time change rate`))))
        (else
          (set `self.Time to change emissive` (- (`self.Time to change emissive`) (* (`GameplayStatics.GetWorldDeltaSeconds`) (`local.Time change rate`))))))
      (`MaterialInstanceDynamic.SetScalarParameterValue` (`self.Emissive light_Around`) "Emissive" (`KismetMathLibrary.Lerp` 5.0 500.0 (`KismetMathLibrary.FClamp` (`self.Time to change emissive`)))))))

(fn `UserConstructionScript`)