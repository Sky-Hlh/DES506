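; Vortex effect actor that can be shown and hidden with a fade, built from a particle component and a cone mesh.
; On BeginPlay it creates a dynamic material instance for the cone.
; Appear activates the particles, reveals the cone and fades its Opacity parameter in via a timeline.
; Disappear deactivates the particles, fades the cone out, and hides it when that timeline finishes.
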(event `self.ReceiveBeginPlay`
  (bind _returnvalue (`PrimitiveComponent.CreateDynamicMaterialInstance` (`self.Cone`) 0 null "None"))
  (set `self.M_Cone` _returnvalue))

(event `Appear`
  (`ActorComponent.SetActive` (`self.P_Vortex`) true false)
  (`SceneComponent.SetVisibility` (`self.Cone`) true false)
  (bind (_direction _newtrack_0) (`Timeline|Timeline_0` :!via `PlayFromStart`)
    (:`Update`
      (`MaterialInstanceDynamic.SetScalarParameterValue` (`self.M_Cone`) "Opacity" (`KismetMathLibrary.Lerp` 0.0 1.0 _newtrack_0)))))

(event `Disappear`
  (`ActorComponent.SetActive` (`self.P_Vortex`) false false)
  (bind (_direction _newtrack_0) (`Timeline|Timeline_1` :!via `PlayFromStart`)
    (:`Update`
      (`MaterialInstanceDynamic.SetScalarParameterValue` (`self.M_Cone`) "Opacity" (`KismetMathLibrary.Lerp` 1.0 0.0 _newtrack_0)))
    (:`Finished`
      (`SceneComponent.SetVisibility` (`self.Cone`) false false))))

(fn `UserConstructionScript`)