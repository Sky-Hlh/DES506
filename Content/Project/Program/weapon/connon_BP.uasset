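; Cannon weapon Blueprint that fires red bullet projectiles from its Firepoint component.
; Firefunction checks CanFire, spawns a Bullet_red at the Firepoint location with zero rotation, and overrides its ProjectileMovement velocity at a fixed speed.
; The shot direction points from the Firepoint toward the world origin rather than along the cannon's facing.
; The event graph and construction script are empty, so nothing in this Blueprint calls Firefunction or sets CanFire.
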(fn `firefunction`
  (if (`self.CanFire`)
    (bind _returnvalue (`|SpawnActorFromClass` "/Game/Project/Program/EnemyAi/NewFolder/bullet_red.bullet_red_C" (`KismetMathLibrary.MakeTransform` (`SceneComponent.K2_GetComponentLocation` (`self.firepoint`))) "Undefined" "OverrideRootScale" null null))
    (set `MovementComponent.Velocity` (* (`KismetMathLibrary.GetDirectionUnitVector` (`SceneComponent.K2_GetComponentLocation` (`self.firepoint`))) 10000.0) (`/Game/Project/Program/EnemyAi/NewFolder/bullet_red.ProjectileMovement` _returnvalue))
    (return)))

(fn `UserConstructionScript`)